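; BP_Door is a locked door that a character unlocks with a matching item and opens by interacting.
; Interact checks the character for the item, and on a match only sets IsOpen and deletes the item.
; Later interactions without the item play a timeline that slides the cube along Z if unlocked.
; If still locked, a DoOnce-guarded thought widget shows the door's text briefly, then removes itself and resets the guard.
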(event `/Game/GameProject/Interfaces/BPI_Interact.Interact`
  (params (Character :type "/Game/GameProject/Character/BP_PlayerCharacter Object Reference"))
  (bind _returnvalue (`/Game/GameProject/Character/BP_PlayerCharacter.IsItem?` Character (`self.Door`)))
  (if _returnvalue
    (set `self.IsOpen?` true)
    (`/Game/GameProject/Character/BP_PlayerCharacter.DeleteItem` Character (`self.Door`))
    (elif (`self.IsOpen?`)
      (bind (_direction `_новая_дорожка_0`) (`Timeline|Шкала времени` :`NewTime` 2.0)
        (:`Update`
          (`SceneComponent.K2_SetRelativeLocation` (`self.Cube`) (`KismetMathLibrary.MakeVector` 0.0 0.0 (`KismetMathLibrary.Lerp` 0.0 250.0 `_новая_дорожка_0`)) false false)))
      (else
        (`/Engine/EditorBlueprintResources/StandardMacros.DoOnce` false :!label _label
          (:`Completed`
            (bind _returnvalue_2 (`|CreateWidget` "/Game/GameProject/Widgets/WBP_Thoughts.WBP_Thoughts_C" null (`self.Thoughts`)))
            (bind _output_get (set `self.DoorThoughts` _returnvalue_2))
            (`UserWidget.AddToViewport` _output_get 0)
            (`KismetSystemLibrary.Delay` 5.0)
            (bind _doorthoughts (`self.DoorThoughts`)
              (:`then`
                (`Widget.RemoveFromParent` _doorthoughts)
                (goto _label :!via `Reset`))
              (:`else`))))))))

(fn `UserConstructionScript`)
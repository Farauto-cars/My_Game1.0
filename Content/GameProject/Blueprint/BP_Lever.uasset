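; BP_Lever is an interactable lever that opens the BP_LeverDoor actors linked to it.
; Interact passes a DoOnce gate, then after a delay calls OpenDoor on every door whose LeverDoor value matches this lever's Levers value.
; In parallel, a FlipFlop alternately plays and reverses a timeline that rolls the Arrow component through a half turn.
; The timeline update resets the gate after a delay, blocking rapid repeat use.
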(event `/Game/GameProject/Interfaces/BPI_Interact.Interact`
  (params (Character :type "/Game/GameProject/Character/BP_PlayerCharacter Object Reference"))
  ;[0 0 0] Взаимодействие с рычагом
  (`/Engine/EditorBlueprintResources/StandardMacros.DoOnce` false :!label _label
    (:`Completed`
      (`|ExecutionSequence`
        (:`then_0`
          (`KismetSystemLibrary.Delay` 1.0)
          (bind _outactors (`GameplayStatics.GetAllActorsOfClass` "/Game/GameProject/Blueprint/BP_LeverDoor.BP_LeverDoor_C"))
          (for _array_element _outactors
            (if (== (`self.Levers`) (`/Game/GameProject/Blueprint/BP_LeverDoor.LeverDoor` _array_element))
              (`/Game/GameProject/Blueprint/BP_LeverDoor.OpenDoor` _array_element))))
        (:`then_1`
          (`/Engine/EditorBlueprintResources/StandardMacros.FlipFlop`
            (:`A`
              (bind (_direction _alpha) (`Timeline|Шкала времени` :!label _label_2)
                (:`Update`
                  (`SceneComponent.K2_SetRelativeRotation` (`self.Arrow`) (`KismetMathLibrary.MakeRotator` (`KismetMathLibrary.Lerp` 0.0 180.0 _alpha)) false false)
                  (`KismetSystemLibrary.Delay` 1.0)
                  (goto _label :!via `Reset`))))
            (:`B`
              (goto _label_2 :!via `Reverse`))))))))

(fn `UserConstructionScript`)
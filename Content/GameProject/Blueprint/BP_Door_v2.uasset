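; Door actor that needs two key items from the interacting character before it slides upward.
; Interact checks both items, swapping each matching key slot's mesh once; holding both sets IsOpen and removes them from the character.
; Missing-item branches play a timeline lifting the Cube if IsOpen.
; Otherwise they show a thought widget for five seconds, gated by a DoOnce that resets after removal.
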(event `self.Interact`
  (params (Character :type "/Game/GameProject/Character/BP_PlayerCharacter Object Reference"))
  (`|ExecutionSequence`
    (:`then_0`
      (bind _returnvalue (`/Game/GameProject/Character/BP_PlayerCharacter.IsItem?` Character (`self.Door`)))
      (if _returnvalue
        (`|ExecutionSequence`
          (:`then_0`
            (`/Engine/EditorBlueprintResources/StandardMacros.DoOnce` false
              (:`Completed`
                (`StaticMeshComponent.SetStaticMesh` (`self.Key1`) "/Game/GameProject/Meshes/key_block.key_block"))))
          (:`then_1`
            (if (and _returnvalue (stale _returnvalue_3)) :!label _label
              (set `self.IsOpen?` true)
              (`/Game/GameProject/Character/BP_PlayerCharacter.DeleteItem` Character (`self.Door`))
              (`/Game/GameProject/Character/BP_PlayerCharacter.DeleteItem` Character (`self.Door2`)))))
        (else
          (if (`self.IsOpen?`) :!label _label_2
            (bind (_direction `_новая_дорожка_0`) (`Timeline|Шкала времени` :`NewTime` 2.0)
              (:`Update`
                (`SceneComponent.K2_SetRelativeLocation` (`self.Cube`) (`KismetMathLibrary.MakeVector` 0.0 0.0 (`KismetMathLibrary.Lerp` 0.0 250.0 `_новая_дорожка_0`)) false false)))
            (else
              (`/Engine/EditorBlueprintResources/StandardMacros.DoOnce` false :!label _label_3
                (:`Completed`
                  (bind _returnvalue_2 (`|CreateWidget` "/Game/GameProject/Widgets/WBP_Thoughts.WBP_Thoughts_C" null (`self.Thoughts`)))
                  (bind _output_get (set `self.DoorThoughts` _returnvalue_2))
                  (`UserWidget.AddToViewport` _output_get 0)
                  (`KismetSystemLibrary.Delay` 5.0)
                  (bind _doorthoughts (`self.DoorThoughts`)
                    (:`then`
                      (`Widget.RemoveFromParent` _doorthoughts)
                      (goto _label_3 :!via `Reset`))
                    (:`else`)))))))))
    (:`then_1`
      (bind _returnvalue_3 (`/Game/GameProject/Character/BP_PlayerCharacter.IsItem?` Character (`self.Door2`)))
      (if _returnvalue_3
        (`|ExecutionSequence`
          (:`then_0`
            (goto _label))
          (:`then_1`
            (`/Engine/EditorBlueprintResources/StandardMacros.DoOnce` false
              (:`Completed`
                (`StaticMeshComponent.SetStaticMesh` (`self.Key2`) "/Game/GameProject/Meshes/key_block.key_block")))))
        (else
          (goto _label_2))))))

(fn `UserConstructionScript`)
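; Item inspection actor that shows a close-up, rotatable copy of an inspectable item with its name.
; Inspect copies the item's mesh, rotation and scale, hides item and character, moves input and view to itself and adds the name widget.
; Both mouse axes feed one combined rotation on the mesh.
; IA_ReadDescription opens a description widget once; IA_Close dismisses it, or otherwise destroys the actor, restoring input and visibility.
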(event `/Game/GameProject/Interfaces/BPI_Inspect.Inspect`
  (params (Character :type "/Game/GameProject/Character/BP_PlayerCharacter Object Reference") (CurrentInspectableItem :type "/Game/GameProject/Blueprint/BP_InspectableItem Object Reference"))
  (bind _returnvalue (`GameplayStatics.GetPlayerController` 0))
  (bind _camera (`self.Camera`))
  (`|ExecutionSequence`
    (:`then_0`
      (set `self.Character` Character)
      (set `self.Current Inspectable Item` CurrentInspectableItem)
      (`|ExecutionSequence`
        (:`then_0`
          (`StaticMeshComponent.SetStaticMesh` (`self.StaticMesh`) (`StaticMeshComponent.StaticMesh` (`/Game/GameProject/Blueprint/BP_InspectableItem.StaticMesh` (`self.Current Inspectable Item`))))
          (`SceneComponent.K2_SetRelativeRotation` (`self.StaticMesh`) (`/Game/GameProject/Blueprint/BP_InspectableItem.ItemRotation` (`self.Current Inspectable Item`)) false false)
          (`SceneComponent.SetRelativeScale3D` (`self.StaticMesh`) (`/Game/GameProject/Blueprint/BP_InspectableItem.ItemScale` (`self.Current Inspectable Item`)))
          (`self.SetActorHiddenInGame` (`self.Current Inspectable Item`) true)
          (`self.SetActorHiddenInGame` (`self.Character`) true))
        (:`then_1`
          (bind _returnvalue_2 (`|CreateWidget` "/Game/GameProject/Widgets/WBP_ItemName.WBP_ItemName_C" null (`/Game/GameProject/Blueprint/BP_InspectableItem.ItemName` (`self.Current Inspectable Item`))))
          (bind _output_get (set `self.WidgetInspect` _returnvalue_2))
          (`UserWidget.AddToViewport` _output_get 0)
          (`self.DisableInput` _returnvalue _returnvalue)
          (`self.EnableInput` _returnvalue))
        (:`then_2`
          (`self.K2_SetActorLocation` (+ (`SceneComponent.K2_GetComponentLocation` _camera) (* (`SceneComponent.GetForwardVector` _camera) 20.0))))))
    (:`then_1`
      (`PlayerController.SetViewTargetWithBlend` (`GameplayStatics.GetPlayerController` 0) self 0.0 "VTBlend_Linear" 0.0 false))))

(event `InputAxisKey|MouseX`
  (params (AxisValue :type "Float (single-precision)"))
  (bind _staticmesh (`self.StaticMesh`))
  (`SceneComponent.K2_SetWorldRotation` _staticmesh (`KismetMathLibrary.ComposeRotators` (`SceneComponent.K2_GetComponentRotation` _staticmesh) (`KismetMathLibrary.MakeRotator` (* (stale `InputAxisKey|MouseY` AxisValue) -3.0) 0.0 (* AxisValue -3.0))) false false :!label _label))

(event `InputAxisKey|MouseY`
  (params (AxisValue :type "Float (single-precision)"))
  (goto _label))

(event `EnhancedInput|/Game/GameProject/Core/EnhancedInput/Action/IA_Close`
  (params (ActionValue :type Boolean) (ElapsedSeconds :type "Float (double-precision)") (TriggeredSeconds :type "Float (double-precision)") (InputAction :type "InputAction Object Reference" :default "/Game/GameProject/Core/EnhancedInput/Action/IA_Close.IA_Close"))
  (bind _returnvalue (`GameplayStatics.GetPlayerController` 0))
  (:`Started`
    (bind _output_get (set `self.IsOpenDescription?` (`self.IsOpenDescription?`)))
    (if _output_get
      (bind _widgetdescription (`self.WidgetDescription`)
        (:`then`
          (`Widget.RemoveFromParent` _widgetdescription)
          (set `self.IsOpenDescription?` false)
          (goto _label_2 :!via `Reset`))
        (:`else`))
      (else
        (`self.K2_DestroyActor`)
        (`self.DisableInput` _returnvalue)
        (`self.EnableInput` _returnvalue _returnvalue)
        (bind _widgetinspect (`self.WidgetInspect`)
          (:`then`
            (`Widget.RemoveFromParent` _widgetinspect)
            (set `self.WidgetInspect` null)
            (`self.SetActorHiddenInGame` (`self.Current Inspectable Item`) false)
            (`self.SetActorHiddenInGame` (`self.Character`) false))
          (:`else`))))))

(event `EnhancedInput|/Game/GameProject/Core/EnhancedInput/Action/IA_ReadDescription`
  (params (ActionValue :type Boolean) (ElapsedSeconds :type "Float (double-precision)") (TriggeredSeconds :type "Float (double-precision)") (InputAction :type "InputAction Object Reference" :default "/Game/GameProject/Core/EnhancedInput/Action/IA_ReadDescription.IA_ReadDescription"))
  (:`Started`
    (set `self.IsOpenDescription?` true)
    (`/Engine/EditorBlueprintResources/StandardMacros.DoOnce` false :!label _label_2
      (:`Completed`
        (bind _returnvalue (`|CreateWidget` "/Game/GameProject/Widgets/WBP_ItemDescription.WBP_ItemDescription_C" null (`/Game/GameProject/Blueprint/BP_InspectableItem.ItemDescription` (`self.Current Inspectable Item`))))
        (bind _output_get (set `self.WidgetDescription` _returnvalue))
        (`UserWidget.AddToViewport` _output_get 0)))))

(fn `UserConstructionScript`)
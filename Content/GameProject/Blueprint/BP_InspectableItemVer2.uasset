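; Inspectable item actor that, when interacted with, blends the camera to itself and moves input from the player controller to the item.
; The read action opens a description widget built from the item's Description, with a DoOnce blocking duplicates.
; The close action first removes an open description and resets the DoOnce.
; With no description open, it returns the view to the player character and restores player controller input.
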(event `self.Interact`
  (params (Character :type "/Game/GameProject/Character/BP_PlayerCharacter Object Reference") (GameInstance :type "Object Object Reference"))
  (bind _returnvalue (`GameplayStatics.GetPlayerController` 0))
  (`|ExecutionSequence`
    (:`then_0`
      (`self.DisableInput` _returnvalue _returnvalue)
      (`self.EnableInput` _returnvalue))
    (:`then_1`
      (`PlayerController.SetViewTargetWithBlend` (`GameplayStatics.GetPlayerController` 0) self 0.0 "VTBlend_Linear" 0.0 false))))

(event `EnhancedInput|/Game/GameProject/Core/EnhancedInput/Action/IA_Close`
  (params (ActionValue :type Boolean) (ElapsedSeconds :type "Float (double-precision)") (TriggeredSeconds :type "Float (double-precision)") (InputAction :type "InputAction Object Reference" :default "/Game/GameProject/Core/EnhancedInput/Action/IA_Close.IA_Close"))
  (bind _returnvalue (`GameplayStatics.GetPlayerController` 0))
  (:`Started`
    (bind _output_get (set `self.IsOpenDescription?` (`self.IsOpenDescription?`)))
    (if _output_get
      (bind _widgetdescription (`self.WidgetDescription`)
        (:`then`
          (`Widget.RemoveFromParent` _widgetdescription)
          (set `self.IsOpenDescription?` false)
          (goto _label :!via `Reset`))
        (:`else`))
      (else
        (`PlayerController.SetViewTargetWithBlend` _returnvalue (`GameplayStatics.GetPlayerCharacter` 0) 0.0 "VTBlend_Linear" 0.0 false)
        (`self.DisableInput` _returnvalue)
        (`self.EnableInput` _returnvalue _returnvalue)))))

(event `EnhancedInput|/Game/GameProject/Core/EnhancedInput/Action/IA_ReadDescription`
  (params (ActionValue :type Boolean) (ElapsedSeconds :type "Float (double-precision)") (TriggeredSeconds :type "Float (double-precision)") (InputAction :type "InputAction Object Reference" :default "/Game/GameProject/Core/EnhancedInput/Action/IA_ReadDescription.IA_ReadDescription"))
  (:`Started`
    (set `self.IsOpenDescription?` true)
    (`/Engine/EditorBlueprintResources/StandardMacros.DoOnce` false :!label _label
      (:`Completed`
        (bind _returnvalue (`|CreateWidget` "/Game/GameProject/Widgets/WBP_ItemDescription.WBP_ItemDescription_C" null (`self.Description`)))
        (bind _output_get (set `self.WidgetDescription` _returnvalue))
        (`UserWidget.AddToViewport` _output_get 0)))))

(fn `UserConstructionScript`)
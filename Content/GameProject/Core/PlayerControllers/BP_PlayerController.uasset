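; Player controller for a first-person character, handling Enhanced Input movement, look, crouch, sprint and interaction.
; BeginPlay adds the game mapping context, caches the possessed BP_PlayerCharacter and creates a crosshair widget.
; Every tick it picks an idle, walk or run camera shake from velocity and line-traces from the camera, showing the crosshair only over BPI_Crosshair actors.
; Interact repeats that short trace and sends InteractMessage to the hit actor.
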(event `self.ReceiveTick`
  (params (DeltaSeconds :type "Float (single-precision)"))
  (bind _crosshair (`self.Crosshair`))
  (bind _playercamera (`/Game/GameProject/Character/BP_PlayerCharacter.PlayerCamera` (`self.As BP Player Character`)))
  (bind _returnvalue (`SceneComponent.K2_GetComponentLocation` _playercamera))
  (`|ExecutionSequence`
    (:`then_0`
      (`self.CameraShake`))
    (:`then_1`
      (`self.Crosshair`
        (:`then`
          (bind (_outhit _returnvalue_2) (`KismetSystemLibrary.LineTraceSingle` _returnvalue (+ _returnvalue (* (`SceneComponent.GetForwardVector` _playercamera) 300.0)) "TraceTypeQuery1"))
          (if _returnvalue_2
            (if (`KismetSystemLibrary.DoesImplementInterface` (`.HitActor` (`GameplayStatics.BreakHitResult` _outhit)) "/Game/GameProject/Interfaces/BPI_Crosshair.BPI_Crosshair_C")
              (if (not (`Widget.IsInViewport` _crosshair))
                (`UserWidget.AddToViewport` _crosshair 0))
              (else
                (`Widget.RemoveFromParent` _crosshair :!label _label)))
            (else
              (goto _label))))
        (:`else`)))))

(event `self.ReceiveBeginPlay`
  (`|ExecutionSequence`
    (:`then_0`
      (`WidgetBlueprintLibrary.SetInputMode_GameOnly` self)
      (set `self.bShowMouseCursor` false)
      (`EnhancedInputSubsystemInterface.AddMappingContext` (subsystem `EnhancedInputLocalPlayerSubsystem`) "/Game/GameProject/Core/EnhancedInput/IMC_Game.IMC_Game" 0 (struct))
      (bind _asbp_player_character (cast `/Game/GameProject/Character/BP_PlayerCharacter` (`self.K2_GetPawn`)))
      (bind _output_get (set `self.As BP Player Character` _asbp_player_character))
      (set `self.Character Movement` (`Character.CharacterMovement` _output_get)))
    (:`then_1`
      (bind _returnvalue (`|CreateWidget` "/Game/GameProject/Widgets/WBP_HUD.WBP_HUD_C"))
      (set `self.Crosshair` _returnvalue))))

(event `EnhancedInput|/Game/GameProject/Core/EnhancedInput/Action/IA_Move`
  (params (ActionValue :type "Vector2D Structure") (ElapsedSeconds :type "Float (double-precision)") (TriggeredSeconds :type "Float (double-precision)") (InputAction :type "InputAction Object Reference" :default "/Game/GameProject/Core/EnhancedInput/Action/IA_Move.IA_Move"))
  (bind (_returnvalue_roll _returnvalue_pitch _returnvalue_yaw) (`KismetMathLibrary.BreakRotator` (`self.GetControlRotation`)))
  (bind (_returnvalue_roll_2 _returnvalue_pitch_2 _returnvalue_yaw_2) (`KismetMathLibrary.BreakRotator` (`self.GetControlRotation`)))
  ;[0 0 0] Передвижение
  (:`Triggered`
    (bind _character_movement (`self.Character Movement`)
      (:`then`
        (`|ExecutionSequence`
          (:`then_0`
            (`PawnMovementComponent.AddInputVector` _character_movement (* (`KismetMathLibrary.GetForwardVector` (`KismetMathLibrary.MakeRotator` 0.0 0.0 _returnvalue_yaw)) ActionValue_Y) false))
          (:`then_1`
            (`PawnMovementComponent.AddInputVector` _character_movement (* (`KismetMathLibrary.GetRightVector` (`KismetMathLibrary.MakeRotator` _returnvalue_roll_2 0.0 _returnvalue_yaw_2)) ActionValue_X) false))))
      (:`else`))))

(event `CameraShake`
  (bind _returnvalue (`GameplayStatics.GetPlayerController` 0))
  (bind _returnvalue_2 (`KismetMathLibrary.VSize` (`self.GetVelocity` (`self.As BP Player Character`))))
  ;[0 0 0] Тряска камеры
  (if (> _returnvalue_2 0.0)
    (if (< _returnvalue_2 450.0)
      (`self.ClientStartCameraShake` :`self` _returnvalue :`Shake` "/Game/GameProject/Blueprint/CameraShake/BP_CameraShakeWalk.BP_CameraShakeWalk_C" :`Scale` 0.5)
      (else
        (`self.ClientStartCameraShake` "/Game/GameProject/Blueprint/CameraShake/BP_CameraShakeRun.BP_CameraShakeRun_C")))
    (else
      (`self.ClientStartCameraShake` :`self` _returnvalue :`Shake` "/Game/GameProject/Blueprint/CameraShake/BP_CameraShakeIdle.BP_CameraShakeIdle_C"))))

(event `EnhancedInput|/Game/GameProject/Core/EnhancedInput/Action/IA_Look`
  (params (ActionValue :type "Vector2D Structure") (ElapsedSeconds :type "Float (double-precision)") (TriggeredSeconds :type "Float (double-precision)") (InputAction :type "InputAction Object Reference" :default "/Game/GameProject/Core/EnhancedInput/Action/IA_Look.IA_Look"))
  ;[0 0 0] Поворот камеры
  (:`Triggered`
    (`self.AddYawInput` ActionValue_X)
    (`self.AddPitchInput` ActionValue_Y)))

(event `EnhancedInput|/Game/GameProject/Core/EnhancedInput/Action/IA_Interact`
  (params (ActionValue :type Boolean) (ElapsedSeconds :type "Float (double-precision)") (TriggeredSeconds :type "Float (double-precision)") (InputAction :type "InputAction Object Reference" :default "/Game/GameProject/Core/EnhancedInput/Action/IA_Interact.IA_Interact"))
  (bind _playercamera (`/Game/GameProject/Character/BP_PlayerCharacter.PlayerCamera` (`self.As BP Player Character`)))
  (bind _returnvalue (`SceneComponent.K2_GetComponentLocation` _playercamera))
  ;[0 0 0] Взаимодействие
  (:`Started`
    (bind (_outhit _returnvalue_2) (`KismetSystemLibrary.LineTraceSingle` _returnvalue (+ _returnvalue (* (`KismetMathLibrary.GetForwardVector` (`SceneComponent.K2_GetComponentRotation` _playercamera)) 300.0)) "TraceTypeQuery1"))
    (if _returnvalue_2
      (message `/Game/GameProject/Interfaces/BPI_Interact.Interact` (`.HitActor` (`GameplayStatics.BreakHitResult` _outhit)) (`self.As BP Player Character`)))))

(event `EnhancedInput|/Game/GameProject/Core/EnhancedInput/Action/IA_Crouch`
  (params (ActionValue :type Boolean) (ElapsedSeconds :type "Float (double-precision)") (TriggeredSeconds :type "Float (double-precision)") (InputAction :type "InputAction Object Reference" :default "/Game/GameProject/Core/EnhancedInput/Action/IA_Crouch.IA_Crouch"))
  (bind _as_bp_player_character (`self.As BP Player Character`))
  ;[0 0 0] Присед
  (:`Triggered`
    (`Character.Crouch` _as_bp_player_character)
    (set `self.IsCrouch?` true))
  (:`Completed`
    (`Character.UnCrouch` _as_bp_player_character)
    (set `self.IsCrouch?` false)))

(event `EnhancedInput|/Game/GameProject/Core/EnhancedInput/Action/IA_Run`
  (params (ActionValue :type "Vector2D Structure") (ElapsedSeconds :type "Float (double-precision)") (TriggeredSeconds :type "Float (double-precision)") (InputAction :type "InputAction Object Reference" :default "/Game/GameProject/Core/EnhancedInput/Action/IA_Run.IA_Run"))
  (bind _charactermovement (`Character.CharacterMovement` (`self.As BP Player Character`)))
  ;[0 0 0] Ускорение
  (:`Triggered`
    (set `CharacterMovementComponent.MaxWalkSpeed` 500.0 _charactermovement))
  (:`Completed`
    (set `CharacterMovementComponent.MaxWalkSpeed` 300.0 _charactermovement)))

(fn `UserConstructionScript`)
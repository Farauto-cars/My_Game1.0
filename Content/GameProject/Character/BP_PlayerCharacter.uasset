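; Player character Blueprint that smooths the camera height when crouching and holds a simple item inventory.
; BeginPlay derives standing and crouched heights from the SpringArm's relative Z.
; Crouch events use the capsule height adjustment to set a start height and target, which Tick interpolates with FInterpTo onto the SpringArm until nearly settled.
; AddItem, IsItem? and DeleteItem add unique items, check membership and remove items.
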(event `self.ReceiveBeginPlay`
  (bind (_relativelocation_x _relativelocation_y _relativelocation_z) (`KismetMathLibrary.BreakVector` (`SceneComponent.RelativeLocation` (`self.SpringArm`))))
  ;[0 0 0] Плавное приседание
  (set `self.CameraLocationStanding` _relativelocation_z)
  (set `self.CameraLocationCrouching` (- (`self.CameraLocationStanding`) 30.0))
  (set `self.CameraLocationCurrent` (`self.CameraLocationStanding`)))

(event `self.ReceiveTick`
  (params (DeltaSeconds :type "Float (single-precision)"))
  ;[0 0 0] Плавное приседание
  (`self.OnTickCrouched`))

(event `self.K2_OnStartCrouch`
  (params (HalfHeightAdjust :type "Float (single-precision)") (ScaledHalfHeightAdjust :type "Float (single-precision)"))
  ;[0 0 0] Плавное приседание
  (set `self.CameraLocationCurrent` (+ ScaledHalfHeightAdjust (`self.CameraLocationStanding`)))
  (set `self.CameraLocationTarget` (`self.CameraLocationCrouching`)))

(event `self.K2_OnEndCrouch`
  (params (HalfHeightAdjust :type "Float (single-precision)") (ScaledHalfHeightAdjust :type "Float (single-precision)"))
  ;[0 0 0] Плавное приседание
  (set `self.CameraLocationCurrent` (- ScaledHalfHeightAdjust (`self.CameraLocationStanding`)))
  (set `self.CameraLocationTarget` (`self.CameraLocationStanding`)))

(event `OnTickCrouched`
  (bind _cameralocationcurrent (`self.CameraLocationCurrent`))
  ;[0 0 0] Плавное приседание
  (if (not (or (`KismetMathLibrary.NearlyEqual_FloatFloat` (`self.CameraLocationStanding`) _cameralocationcurrent) (`KismetMathLibrary.NearlyEqual_FloatFloat` (`self.CameraLocationCrouching`) _cameralocationcurrent)))
    (set `self.CameraLocationCurrent` (`KismetMathLibrary.FInterpTo` (`self.CameraLocationCurrent`) (`self.CameraLocationTarget`) (`GameplayStatics.GetWorldDeltaSeconds`) 5.0))
    (`SceneComponent.K2_SetRelativeLocation` (`self.SpringArm`) (`KismetMathLibrary.MakeVector` 0.0 0.0 (`self.CameraLocationCurrent`)) false false)))

(fn `AddItem`
  (params (NewItem :type "Name (by ref)"))
  (`KismetArrayLibrary.Array_AddUnique` (`self.Item`) NewItem))

(fn `DeleteItem`
  (params (Item :type "Name (by ref)"))
  (`KismetArrayLibrary.Array_RemoveItem` (`self.Item`) Item))

(fn `IsItem?`
  (params (ItemToFind :type "Name (by ref)"))
  (returns (ReturnValue :type Boolean))
  (return (`KismetArrayLibrary.Array_Contains` (`self.Item`) ItemToFind)))

(fn `UserConstructionScript`)